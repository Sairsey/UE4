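; Actor Blueprint that moves its Mesh along its Spline component at a constant 100 units per second.
; Each Tick adds delta time to Dist, which is scaled into a distance for sampling the spline's world transform.
; The mesh takes that transform, with a -90 degree Z-axis rotation combined into its orientation.
; Dist grows without any looping or reset, and the move does not sweep for collision.
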(event `self.ReceiveTick`
  (params (DeltaSeconds :type "Float (single-precision)"))
  (bind _output_get (set `self.Dist` (+ DeltaSeconds (`self.Dist`))))
  (`SceneComponent.K2_SetWorldTransform` (`self.Mesh`) (`KismetMathLibrary.MakeTransform` (.location (`SplineComponent.GetTransformAtDistanceAlongSpline` (`self.Spline`) (* _output_get 100.0) "World" false)) (`KismetMathLibrary.ComposeRotators` (.rotation (`SplineComponent.GetTransformAtDistanceAlongSpline` (`self.Spline`) (* _output_get 100.0) "World" false)) (`KismetMathLibrary.RotatorFromAxisAndAngle` (0.0 0.0 1.0) -90.0)) (.scale (`SplineComponent.GetTransformAtDistanceAlongSpline` (`self.Spline`) (* _output_get 100.0) "World" false))) false false))

(fn `UserConstructionScript`)