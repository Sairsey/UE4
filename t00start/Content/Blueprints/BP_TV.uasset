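; BP_TV is a television actor that makes only the TV nearest the player appear switched on.
; BeginPlay sets its two meshes from IsTurnedOff, but Tick then overrides that by calling FindNearest1.
; Each instance scans every BP_TV each frame, measuring distance to the first BP_Player1.
; It shows all TVs as off, then flips the closest to on, using components tagged TV_ON and TV_OFF.
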(event `self.ReceiveBeginPlay`
  (bind _isturnedoff (`self.IsTurnedOff`))
  (`SceneComponent.SetVisibility` (`self.StaticMesh`) _isturnedoff true)
  (`SceneComponent.SetVisibility` (`self.StaticMesh2`) (not _isturnedoff) true))

(event `self.ReceiveTick`
  (params (DeltaSeconds :type "Float (single-precision)"))
  (`self.Find nearest1`))

(fn `Find nearest1`
  (bind _nearest (`self.nearest`))
  (bind _outactors (`GameplayStatics.GetAllActorsOfClass` "/Game/Blueprints/BP_Player1.BP_Player1_C"))
  (bind _outactors_2 (`GameplayStatics.GetAllActorsOfClass` "BP_TV_C"))
  (bind _output (`|GetArrayItem` _outactors_2))
  (bind _output_2 (`|GetArrayItem` _outactors))
  (set `self.lenght` (`KismetMathLibrary.VSize` (- (`self.K2_GetActorLocation` _output) (`self.K2_GetActorLocation` _output_2))))
  (set `self.nearest` _output)
  (for _array_element _outactors_2
    (bind _asscene_component (cast `SceneComponent` (`|GetArrayItem` (`self.GetComponentsByTag` _array_element "/Script/Engine.ActorComponent" "TV_ON"))))
    (bind _asscene_component_2 (cast `SceneComponent` (`|GetArrayItem` (`self.GetComponentsByTag` _array_element "/Script/Engine.ActorComponent" "TV_OFF"))))
    (bind _returnvalue (`KismetMathLibrary.VSize` (- (`self.K2_GetActorLocation` _output_2) (`self.K2_GetActorLocation` _array_element))))
    (if (>= (`self.lenght`) _returnvalue)
      (set `self.lenght` _returnvalue)
      (set `self.nearest` _array_element))
    (`SceneComponent.SetVisibility` _asscene_component false false)
    (`SceneComponent.SetVisibility` _asscene_component_2 true false))
  (bind _asscene_component_3 (cast `SceneComponent` (`|GetArrayItem` (`self.GetComponentsByTag` _nearest "/Script/Engine.ActorComponent" "TV_ON"))))
  (bind _asscene_component_4 (cast `SceneComponent` (`|GetArrayItem` (`self.GetComponentsByTag` _nearest "/Script/Engine.ActorComponent" "TV_OFF"))))
  (`SceneComponent.SetVisibility` _asscene_component_3 true false)
  (`SceneComponent.SetVisibility` _asscene_component_4 false false))

(fn `UserConstructionScript`)